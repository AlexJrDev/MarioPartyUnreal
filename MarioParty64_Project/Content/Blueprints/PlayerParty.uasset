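; Player pawn for a party board game that rolls 1 to 10 and walks tile to tile through neighbour links.
; The dice loop steps along the current direction, using timelines to lerp position and rotation, with tiles gating entry and able to chain moves.
; When a roll ends, direction tiles poll for a valid input if several exits exist, then resume movement, while coin tiles add or subtract coins.
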(event Custom|MoveTo
  (params (TileToMove :type Tile%20Object%20Reference))
  ;[0.7813 0 1] Player movement
  (Utilities|IsValid TileToMove
    (:Is%20Valid
      (if (Default|CanPlayerEnter TileToMove self (Variables|Default|GetCurrentTile))
        (Variables|Default|SetTargetTile (Variables|Default|GetCurrentTile))
        (bind _moveto (Timeline|Move PlayFromStart)
          (:Update
            (Variables|Default|SetIsWalking true)
            (Transformation|SetActorLocation (Math|Vector|Lerp(Vector) (Transformation|GetActorLocation (Variables|Default|GetCurrentTile)) (Transformation|GetActorLocation TileToMove) _moveto) false false))
          (:Finished
            (Variables|Default|SetIsWalking false)
            (Variables|Default|SetTemp (Variables|Default|GetCurrentTile))
            (Variables|Default|SetCurrentTile TileToMove)
            (bind _output_get (Variables|Default|SetTargetTile (Default|GetNextTile (Variables|Default|GetCurrentTile) self (Variables|Default|GetTemp))))
            (Utilities|IsValid _output_get
              (:Is%20Valid
                (if (Default|CanPlayerEnter _output_get self (Variables|Default|GetCurrentTile))
                  (CallFunction|Moveto (Variables|Default|GetTargetTile))))
              (:Is%20Not%20Valid
                (Variables|Default|SetTargetTile 0)))
            (Default|OnEnter (Variables|Default|GetCurrentTile) self (Variables|Default|GetTemp))))))))

(event Custom|RotateToDirection
  (params (Direction :type Direction%20Object%20Reference))
  ;[0 1 0.8125] Player Rotation
  (Utilities|IsValid Direction
    (:Is%20Valid
      (Variables|Default|SetTargetDirection Direction)
      (bind _newtrack_0 (Timeline|Rotate PlayFromStart)
        (:Update
          (Transformation|SetActorRotation (Math|Rotator|Lerp(Rotator) (Variables|/Game/Blueprints/Direction.Direction_C|GetRotation (Variables|Default|GetCurrentDirection)) (Variables|/Game/Blueprints/Direction.Direction_C|GetRotation (Variables|Default|GetTargetDirection)) _newtrack_0)))
        (:Finished
          (bind _output_get (Variables|Default|SetCurrentDirection (Variables|Default|GetTargetDirection)))
          (Variables|Default|SetTargetDirection _output_get))))))

(event Input|ActionEvents|InputActionDice
  (params (Key :type Key%20Structure :default "None"))
  ;[1 0.9844 0] Dice Movement
  (:Pressed
    (if (not (Variables|Default|GetIsMoving))
      (Variables|Default|SetIsMoving true)
      (Variables|Default|SetMoveIndex (Math|Random|RandomIntegerinRange 1 10))
      (if (== (Variables|Default|GetMoveIndex) 0) :!label _label
        (Variables|Default|SetTargetDirection (Variables|Default|GetEmptyDirection) :!label _label_2)
        (if (== (Utilities|GetClass (Variables|Default|GetCurrentTile)) "/Game/Blueprints/DirectionTile.DirectionTile_C")
          (bind _keys (Utilities|Map|Keys (Variables|/Game/Blueprints/Tile.Tile_C|GetValidMoveDirections (Variables|Default|GetCurrentTile))))
          (if (== (Utilities|Array|Length _keys) 1) :!label _label_3
            (Variables|Default|SetTargetDirection (Utilities|Array|Get(acopy) _keys))
            (Variables|Default|SetCanMove true :!label _label_4)
            (Variables|Default|SetCurrentDirection (Variables|Default|GetTargetDirection))
            (CallFunction|Moveto (.Value (Utilities|Map|Find (Variables|/Game/Blueprints/Tile.Tile_C|GetNeighbours (Variables|Default|GetCurrentTile)) (Variables|Default|GetCurrentDirection))) :!label _label_5)
            (CallFunction|RotatetoDirection (Variables|Default|GetCurrentDirection))
            (Utilities|FlowControl|Delay 0.2)
            (goto _label)
            (else
              (Variables|Default|SetDirectionSelected false)
              (for _array_element _keys
                (if (== (Variables|Default|GetTargetDirection) _array_element)
                  (if (not (Variables|Default|GetDirectionSelected))
                    (Variables|Default|SetDirectionSelected true)
                    (goto _label_4))))
              (Utilities|FlowControl|Delay 0.1)
              (if (not (Variables|Default|GetDirectionSelected))
                (goto _label_3))))
          (else
            (Variables|Default|SetIsMoving false)
            (if (== (Utilities|GetClass (Variables|Default|GetCurrentTile)) "/Game/Blueprints/CoinTile.CoinTile_C")
              (bind _output_get (Variables|Default|SetCoins (+ (Variables|Default|GetCoins) 3)))
              (Development|PrintString (Utilities|String|Append "Ganaste 3 Monedas tienes" (Utilities|String|ToString(Integer) _output_get)))
              (elif (== (Utilities|GetClass (Variables|Default|GetCurrentTile)) "/Game/Blueprints/LoseCoins.LoseCoins_C")
                (bind _output_get_2 (Variables|Default|SetCoins (- (Variables|Default|GetCoins) 3)))
                (Development|PrintString (Utilities|String|Append "Perdiste 3 Monedas tienes" (Utilities|String|ToString(Integer) _output_get_2)))))))
        (elif (Variables|Default|GetCanMove)
          (Development|PrintString (Utilities|String|ToString(Integer) (Variables|Default|GetMoveIndex)))
          (Math|Integer|DecrementInt (Variables|Default|GetMoveIndex)
            (:%20%20
              (Utilities|IsValid (Variables|Default|GetTargetTile)
                (:Is%20Not%20Valid
                  (Utilities|IsValid (.Value (Utilities|Map|Find (Variables|/Game/Blueprints/Tile.Tile_C|GetNeighbours (Variables|Default|GetCurrentTile)) (Variables|Default|GetCurrentDirection)))
                    (:Is%20Valid
                      (goto _label_5)))))))
          (else
            (goto _label_2)))))))

(event Input|ActionEvents|InputActionMoveLeft
  (params (Key :type Key%20Structure :default "None"))
  ;[0 1 0.03906] Player Map Input
  (:Pressed
    (Variables|Default|SetTargetDirection "/Game/Blueprints/Left.Left")))

(event Input|ActionEvents|InputActionMoveRight
  (params (Key :type Key%20Structure :default "None"))
  ;[0 1 0.03906] Player Map Input
  (:Pressed
    (Variables|Default|SetTargetDirection "/Game/Blueprints/Right.Right")))

(event Input|ActionEvents|InputActionMoveUp
  (params (Key :type Key%20Structure :default "None"))
  ;[0 1 0.03906] Player Map Input
  (:Pressed
    (Variables|Default|SetTargetDirection "/Game/Blueprints/Up.Up")))

(event Input|ActionEvents|InputActionMoveDown
  (params (Key :type Key%20Structure :default "None"))
  ;[0 1 0.03906] Player Map Input
  (:Pressed
    (Variables|Default|SetTargetDirection "/Game/Blueprints/Down.Down")))

(fn ConstructionScript)