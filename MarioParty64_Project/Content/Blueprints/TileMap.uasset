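; TileMap is a grid actor that owns the level's tiles and places the PlayerParty on its spawn tile and facing at BeginPlay.
; Tiles live in a flat row-major array, with helpers for coordinate conversion, bounds and border checks, lookup and replacement.
; ResetMap rebuilds the grid by spawning attached border and fill tiles 100 units apart, rows along world X, then has each tile find its neighbours.
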(event EventBeginPlay
  (bind _returnvalue (Game|Player|GetPlayerPawn 0))
  (Transformation|SetActorLocation _returnvalue (Transformation|GetActorLocation (Variables|Default|GetPlayerSpawnTile)) false false)
  (Transformation|SetActorRotation _returnvalue (Variables|/Game/Blueprints/Direction.Direction_C|GetRotation (Variables|Default|GetPlayerSpawnDirection)))
  (bind _asplayer_party (Utilities|Casting|CastToPlayerParty _returnvalue))
  (Variables|/Game/Blueprints/PlayerParty.PlayerParty_C|SetCurrentTile _asplayer_party (Variables|Default|GetPlayerSpawnTile))
  (Variables|/Game/Blueprints/PlayerParty.PlayerParty_C|SetCurrentDirection _asplayer_party (Variables|Default|GetPlayerSpawnDirection)))

(fn ConstructionScript)

(fn CoordtoIndex
  (params (Coord :type Coord%20Structure))
  (return (+ (.x Coord) (* (.y Coord) (Variables|Default|GetWidth)))))

(fn IndextoCoord
  (params (Index :type Integer))
  (bind _width (Variables|Default|GetWidth))
  (return (Utilities|Struct|MakeCoord (Math|Integer|%(Integer) Index _width) (/ Index _width))))

(fn IsCoordBorder
  (params (Coord :type Coord%20Structure))
  (return (Math|Boolean|ORBoolean (== (- (Variables|Default|GetWidth) 1) (.x Coord)) (== (.x Coord) 0) (== (.y Coord) 0) (== (- (Variables|Default|GetHeight) 1) (.y Coord)))))

(fn IsCoordinRange
  (params (Coord :type Coord%20Structure))
  (return (not (Math|Boolean|ORBoolean (>= (.x Coord) (Variables|Default|GetWidth)) (< (.x Coord) 0) (< (.y Coord) 0) (>= (.y Coord) (Variables|Default|GetHeight))))))

(fn GetTileatCoord
  (params (Coord :type Coord%20Structure))
  (return (Utilities|Array|Get(acopy) (Variables|Default|GetTiles) (CallFunction|CoordtoIndex Coord))))

(fn ResetMap
  (bind _tiles (Variables|Default|GetTiles))
  (for _array_element _tiles
    (Utilities|IsValid _array_element
      (:Is%20Valid
        (Actor|DestroyActor _array_element))))
  (Utilities|Array|Clear _tiles)
  (for _index (range 0 (- (Variables|Default|GetHeight) 1)) ; Y
    (for _index_2 (range 0 (- (Variables|Default|GetWidth) 1)) ; X
      (bind _returnvalue (Game|SpawnActorfromClass (select (CallFunction|IsCoordBorder (Utilities|Struct|MakeCoord _index_2 _index)) (Variables|Default|GetBorderTileType) (Variables|Default|GetFillTileType)) (Math|Transform|MakeTransform (Math|Vector|MakeVector (* _index 1e+02) (* _index_2 1e+02) 0.0) "0, 0, 0" "1,1,1") "Undefined" 0 (Utilities|Struct|MakeCoord _index_2 _index) 0 self (select (CallFunction|IsCoordBorder (Utilities|Struct|MakeCoord _index_2 _index)) (Variables|Default|GetBorderTileType) (Variables|Default|GetFillTileType)) 0))
      (Utilities|Array|Add (Variables|Default|GetTiles) _returnvalue)
      (Transformation|AttachActorToActor _returnvalue self "None" "KeepWorld" "KeepWorld" "KeepWorld" true)))
  (for _array_element_2 (Variables|Default|GetTiles)
    (Default|FindNeighbours _array_element_2)))

(fn ReplaceTile
  (params (NewTile :type Tile%20Object%20Reference))
  (Utilities|Array|SetArrayElem (Variables|Default|GetTiles) (CallFunction|CoordtoIndex (Variables|/Game/Blueprints/Tile.Tile_C|GetCoord NewTile)) NewTile))