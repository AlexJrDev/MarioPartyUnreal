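; DirectionTile is a grid tile Blueprint that works out which directions a player may move from it.
; On BeginPlay it fills ValidMoveDirections with either a forced direction, without a target tile, or every neighbour whose CanPlayerEnter passes.
; Its own CanPlayerEnter always returns true.
; OnEnter is empty, as the logic that stops the pawn and removes the opposite direction is disconnected.
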(event EventBeginPlay
  ;[0 1 0.8359] Calculate Posible Tiles
  (if (Variables|Default|GetUseForceDirection)
    (Utilities|Map|Add (Variables|Default|GetValidMoveDirections) (Variables|Default|GetForceDirection) 0)
    (else
      (bind _values (Utilities|Map|Values (Variables|Default|GetNeighbours)))
      (for (_array_element _array_index) _values
        (if (CallFunction|CanPlayerEnter _array_element)
          (bind _keys (Utilities|Map|Keys (Variables|Default|GetNeighbours)))
          (Utilities|Map|Add (Variables|Default|GetValidMoveDirections) (Utilities|Array|Get(acopy) _keys _array_index) _array_element))))))

(event EventOnEnter
  (params (PlayerPawn :type Player%20Party%20Object%20Reference) (FromTile :type Tile%20Object%20Reference))
  ;[1 0.2109 0] Remove Opposite Tile
)

(fn ConstructionScript
  (|CallParentFunction))

(fn CanPlayerEnter
  (params (PlayerPawn :type Player%20Party%20Object%20Reference) (TileFrom :type Tile%20Object%20Reference))
  (return true))